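; Behavior tree task that picks the next patrol waypoint for an AI-controlled ThirdPersonCharacter.
; It reads the pawn's PatrolPoints array and writes the entry at the Blackboard WayPointIndex into the Waypoint key.
; It then advances the index with a modulo wrap, so the route loops.
; The task finishes reporting failure, and a failed pawn cast stops GetPatrolPoints before the array is set.
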(event `self.ReceiveExecuteAI`
  (params (OwnerController :type "AIController Object Reference") (ControlledPawn :type "Pawn Object Reference"))
  (`self.Get Patrol Points` ControlledPawn)
  (bind _index (`self.Set Next WayPoint` null))
  (`self.Cicle Index` _index)
  (`self.FinishExecute` false))

(fn `Cicle Index`
  (params (Index :type Integer))
  (`BTFunctionLibrary.SetBlackboardValueAsInt` (`self.WayPointIndex`) (mod (+ Index 1) (`KismetArrayLibrary.Array_Length` (`self.Patrol Points`)))))

(fn `Get Patrol Points`
  (params (Object :type "Object Object Reference"))
  (bind _asthird_person_character (cast `/Game/ThirdPersonCPP/Blueprints/ThirdPersonCharacter` Object))
  (set `self.Patrol Points` (`/Game/ThirdPersonCPP/Blueprints/ThirdPersonCharacter.PatrolPoints` _asthird_person_character)))

(fn `Set Next WayPoint`
  (params (Object :type "Object Object Reference"))
  (returns (Index :type Integer))
  (bind _returnvalue (`BTFunctionLibrary.GetBlackboardValueAsInt` (`self.WayPointIndex`)))
  (`BTFunctionLibrary.SetBlackboardValueAsObject` (`self.Waypoint`) (`|GetArrayItem` (`self.Patrol Points`) _returnvalue))
  (return _returnvalue))